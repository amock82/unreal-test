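; Target actor that falls over when hit by a player missile and pops back up shortly after.
; On overlap with an actor tagged both "플레이어" (player) and "미사일" (missile), it destroys that actor and snaps its own pitch down to lie flat.
; The Sphere's overlap events stay off during a short Delay, then return as the pitch resets, so the target cannot be hit while down.
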(event EventBeginPlay)

(event Collision|EventActorBeginOverlap
  (params (OtherActor :type Actor%20Object%20Reference))
  (bind _returnvalue (Transformation|GetActorRotation))
  (bind _returnvalue_2 (Transformation|GetActorRotation))
  (bind (_roll _pitch _yaw) (Math|Rotator|BreakRotator _returnvalue_2))
  (bind (_roll_2 _pitch_2 _yaw_2) (Math|Rotator|BreakRotator _returnvalue))
  (if (and (Actor|ActorHasTag OtherActor "플레이어") (Actor|ActorHasTag OtherActor "미사일"))
    (Actor|DestroyActor OtherActor)
    (Variables|/Script/Engine.PrimitiveComponent|SetbGenerateOverlapEvents (Variables|Default|GetSphere) false)
    (Transformation|SetActorRotation (Math|Rotator|MakeRotator _roll -9e+01 _yaw))
    (Utilities|FlowControl|Delay 0.5)
    (Transformation|SetActorRotation (Math|Rotator|MakeRotator _roll_2 0.0 _yaw_2))
    (Variables|/Script/Engine.PrimitiveComponent|SetbGenerateOverlapEvents (Variables|Default|GetSphere) true)))

(event EventTick
  (params (DeltaSeconds :type Float%20%28single-precision%29)))

(event Collision|EventActorEndOverlap
  (params (OtherActor :type Actor%20Object%20Reference)))

(fn ConstructionScript)