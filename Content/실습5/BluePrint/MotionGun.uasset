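; MotionGun is an actor, apparently a gun, whose Base component sweeps back and forth in yaw.
; Tick calls RotateBase, which uses a two-value State to pick the turn direction and flips it when GetBaseZAngle passes 45 degrees either side of zero.
; A BaseLocalRotation helper applies the local yaw step, scaled by delta time and RotSpeed for frame-rate-independent motion.
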(event EventBeginPlay)

(event Collision|EventActorBeginOverlap
  (params (OtherActor :type Actor%20Object%20Reference)))

(event EventTick
  (params (DeltaSeconds :type Float%20%28single-precision%29))
  (CallFunction|RotateBase DeltaSeconds))

(fn ConstructionScript)

(fn RotateBase
  (params (delta%20second :type Float%20%28single-precision%29))
  (LocalVariables|Setdelta%20Sec delta%20second)
  (if (== (Variables|Default|Getstate) 0)
    (Utilities|BaseLocalRotation 1.0 (LocalVariables|Getdelta%20Sec)
      (:출력실행
        (if (>= (Utilities|GetBaseZAngle) 45.0)
          (Variables|Default|Setstate 1))))
    (else
      (Utilities|BaseLocalRotation -1.0 (LocalVariables|Getdelta%20Sec)
        (:출력실행
          (if (<= (Utilities|GetBaseZAngle) -45.0)
            (Variables|Default|Setstate 0)))))))