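; SiegeEngine is a player-controlled siege engine that drives along its facing direction and turns by input.
; The move axis adds forward-vector movement unless it is attacking, while the turn axis adds controller yaw scaled by RotSpeed and frame time.
; Press and release actions set forward, backward and attack state flags, with only the attack flag read here, to block movement.
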(event EventBeginPlay)

(event Collision|EventActorBeginOverlap
  (params (OtherActor :type Actor%20Object%20Reference)))

(event EventTick
  (params (DeltaSeconds :type Float%20%28single-precision%29)))

(event Input|ActionEvents|InputAction이동액션(앞)
  (params (Key :type Key%20Structure :default "None"))
  (:Pressed
    (Variables|Default|SetisMovingForward true))
  (:Released
    (Variables|Default|SetisMovingForward false)))

(event Input|ActionEvents|InputAction이동액션(뒤)
  (params (Key :type Key%20Structure :default "None"))
  (:Pressed
    (Variables|Default|SetisMovingBack true))
  (:Released
    (Variables|Default|SetisMovingBack false)))

(event Input|ActionEvents|InputAction공격액션
  (params (Key :type Key%20Structure :default "None"))
  (:Pressed
    (Variables|Default|SetisAttacking true))
  (:Released
    (Variables|Default|SetisAttacking false)))

(event Input|AxisEvents|InputAxis이동
  (params (AxisValue :type Float%20%28single-precision%29))
  (if (not (Variables|Default|GetisAttacking))
    (Pawn|Input|AddMovementInput (Transformation|GetActorForwardVector) AxisValue false)))

(event Input|AxisEvents|InputAxis회전
  (params (AxisValue :type Float%20%28single-precision%29))
  (Pawn|Input|AddControllerYawInput (* AxisValue (Variables|Default|GetrotSpeed) (Utilities|Time|GetWorldDeltaSeconds))))

(fn ConstructionScript)