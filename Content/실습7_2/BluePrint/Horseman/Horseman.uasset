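; Horseman is a melee combat unit that fights actors tagged RedTeam with a spear.
; Its Boundary overlap sets the target and attacking flag, and Tick keeps it facing that target.
; A Spear overlap deals damage and switches off its own overlap events; EnableCollider restores them but is not called here.
; Damage lowers Hp and turns a survivor toward its attacker, while OnDeath destroys the actor without being called here.
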(event OnComponentBeginOverlap(Boundary)
  (params (OverlappedComponent :type Primitive%20Component%20Object%20Reference) (OtherActor :type Actor%20Object%20Reference) (OtherComp :type Primitive%20Component%20Object%20Reference) (OtherBodyIndex :type Integer) (bFromSweep :type Boolean) (SweepResult :type Hit%20Result%20Structure%20%28by%20ref%29))
  (if (Actor|ActorHasTag OtherActor "RedTeam")
    (Variables|Default|Settarget OtherActor)
    (Variables|Default|SetisAttacking true)))

(event OnComponentEndOverlap(Boundary)
  (params (OverlappedComponent :type Primitive%20Component%20Object%20Reference) (OtherActor :type Actor%20Object%20Reference) (OtherComp :type Primitive%20Component%20Object%20Reference) (OtherBodyIndex :type Integer))
  (if (Actor|ActorHasTag OtherActor "RedTeam")
    (Variables|Default|SetisAttacking false)))

(event OnComponentBeginOverlap(Spear)
  (params (OverlappedComponent :type Primitive%20Component%20Object%20Reference) (OtherActor :type Actor%20Object%20Reference) (OtherComp :type Primitive%20Component%20Object%20Reference) (OtherBodyIndex :type Integer) (bFromSweep :type Boolean) (SweepResult :type Hit%20Result%20Structure%20%28by%20ref%29))
  (if (Actor|ActorHasTag OtherActor "RedTeam")
    (CallFunction|DisableCollider)
    (Game|Damage|ApplyDamage OtherActor 1e+02 0 self "/Script/Engine.DamageType")))

(event EventBeginPlay)

(event Game|Damage|EventAnyDamage
  (params (Damage :type Float%20%28single-precision%29) (DamageType :type Damage%20Type%20Object%20Reference) (InstigatedBy :type Controller%20Object%20Reference) (DamageCauser :type Actor%20Object%20Reference))
  (bind _output_get (Variables|Default|Sethp (- (Variables|Default|Gethp) Damage)))
  (if (> _output_get 0.0)
    (CallFunction|Lookat self (Pawn|GetControlledPawn InstigatedBy))))

(event EventTick
  (params (DeltaSeconds :type Float%20%28single-precision%29))
  (if (Variables|Default|GetisAttacking)
    (CallFunction|Lookat self (Variables|Default|Gettarget))))

(fn ConstructionScript)

(fn EnableCollider
  (Variables|/Script/Engine.PrimitiveComponent|SetbGenerateOverlapEvents (Variables|Default|GetSpear) true))

(fn DisableCollider
  (Variables|/Script/Engine.PrimitiveComponent|SetbGenerateOverlapEvents (Variables|Default|GetSpear) false))

(fn OnDeath
  (Actor|DestroyActor))