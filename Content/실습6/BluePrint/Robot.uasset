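; Robot is a player-driven Blueprint that moves, turns and animates its wheels.
; The 이동 (move) axis offsets it along local forward without sweep, and 회전 (rotate) yaws it, both scaled by speed and delta time.
; Tick spins WheelsPivot in proportion to the current move input.
; Zoom in and out actions shorten or lengthen the SpringArm in fixed, unclamped steps.
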(event EventBeginPlay)

(event Collision|EventActorBeginOverlap
  (params (OtherActor :type Actor%20Object%20Reference)))

(event EventTick
  (params (DeltaSeconds :type Float%20%28single-precision%29))
  (Transformation|AddLocalRotation (Variables|Default|GetWheelsPivot) (* "-1.000000, 0, 0" (* DeltaSeconds (Input|AxisValues|Get이동) (Variables|Default|GetwheelsRotSpeed))) false false))

(event Input|ActionEvents|InputAction카메라줌인
  (params (Key :type Key%20Structure :default "None"))
  (:Pressed
    (Variables|/Script/Engine.SpringArmComponent|SetTargetArmLength (Variables|Default|GetSpringArm) (+ (Variables|/Script/Engine.SpringArmComponent|GetTargetArmLength (Variables|Default|GetSpringArm)) -3e+01))))

(event Input|ActionEvents|InputAction카메라줌아웃
  (params (Key :type Key%20Structure :default "None"))
  (:Pressed
    (Variables|/Script/Engine.SpringArmComponent|SetTargetArmLength (Variables|Default|GetSpringArm) (+ (Variables|/Script/Engine.SpringArmComponent|GetTargetArmLength (Variables|Default|GetSpringArm)) 3e+01))))

(event Input|AxisEvents|InputAxis이동
  (params (AxisValue :type Float%20%28single-precision%29))
  (Transformation|AddActorLocalOffset (* "1.000000, 0, 0" (* AxisValue (Variables|Default|Getspeed) (Utilities|Time|GetWorldDeltaSeconds))) false false))

(event Input|AxisEvents|InputAxis회전
  (params (AxisValue :type Float%20%28single-precision%29))
  (Transformation|AddActorLocalRotation (* "0.000000,1.000000,0.000000" (* AxisValue (Variables|Default|GetrotSpeed) (Utilities|Time|GetWorldDeltaSeconds))) false false))

(fn ConstructionScript)