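; FootMan is a player-controlled Character Blueprint for a footman with walking, turning, jumping and attacking.
; Axis inputs add movement along the actor's forward vector and yaw the controller by RotSpeed scaled with delta seconds.
; Move and attack action inputs play looping walk or attack animations directly on the mesh, returning to idle on release, with no Animation Blueprint state logic.
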(event EventBeginPlay)

(event Collision|EventActorBeginOverlap
  (params (OtherActor :type Actor%20Object%20Reference)))

(event EventTick
  (params (DeltaSeconds :type Float%20%28single-precision%29)))

(event Input|ActionEvents|InputAction점프
  (params (Key :type Key%20Structure :default "None"))
  (:Pressed
    (Character|Jump)))

(event Input|ActionEvents|InputAction이동액션
  (params (Key :type Key%20Structure :default "None"))
  (:Pressed
    (Components|Animation|PlayAnimation (Variables|Character|GetMesh) "/Game/실습7/Animation/Footman_Walk.Footman_Walk" true))
  (:Released
    (Components|Animation|PlayAnimation (Variables|Character|GetMesh) "/Game/실습7/Animation/Footman_Idle.Footman_Idle" true)))

(event Input|ActionEvents|InputAction공격액션
  (params (Key :type Key%20Structure :default "None"))
  (:Pressed
    (Components|Animation|PlayAnimation (Variables|Character|GetMesh) "/Game/실습7/Animation/Footman_Attack01.Footman_Attack01" true))
  (:Released
    (Components|Animation|PlayAnimation (Variables|Character|GetMesh) "/Game/실습7/Animation/Footman_Idle.Footman_Idle" true)))

(event Input|AxisEvents|InputAxis이동
  (params (AxisValue :type Float%20%28single-precision%29))
  (Pawn|Input|AddMovementInput (* (Transformation|GetActorForwardVector) AxisValue) 1.0 false))

(event Input|AxisEvents|InputAxis회전
  (params (AxisValue :type Float%20%28single-precision%29))
  (Pawn|Input|AddControllerYawInput (* AxisValue (Variables|Default|GetrotSpeed) (Utilities|Time|GetWorldDeltaSeconds))))

(fn ConstructionScript)